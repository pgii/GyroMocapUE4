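; SensorController applies gyro sensor orientation data to a TestSphere actor, apparently as a rotation test.
; GyroDataReceive passes sensor and quaternion through RotateSphere to UpdateTestSphereRotation, which ignores sensors other than CurrentSensor.
; The quaternion becomes a rotator, and RInterpTo smooths toward it using stored delta time and speed variables rather than frame delta.
; QuatPrintString is a debug print helper that nothing here calls.
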(event Custom|RotateSphere
  (params (GyroSensor :type GyroSensorEnum%20Enum :default "NewEnumerator0") (Quat :type Quat%20Structure))
  ;[0.05517 0.1 1] BoneRotation
  (CallFunction|UpdateTestSphereRotation GyroSensor Quat (Variables|Default|GetSmoothDeltaTime) (Variables|Default|GetSmoothInterpSpeed)))

(event Custom|GyroDataReceive
  (params (GyroSensor :type GyroSensorEnum%20Enum :default "NewEnumerator0") (GyroQuaternion :type Quat%20Structure))
  ;[1 0 0.5519] Gyro Data Receive
  (CallFunction|RotateSphere GyroSensor GyroQuaternion))

(fn ConstructionScript)

(fn QuatPrintString
  (params (Quat :type Quat%20Structure) (Color :type Linear%20Color%20Structure))
  (bind (_x _y _z _w) (Utilities|Struct|BreakQuat Quat))
  (Development|PrintString (Utilities|String|Append (Utilities|String|ToString(Float) _x) " | " (Utilities|String|ToString(Float) _y) " | " (Utilities|String|ToString(Float) _z) " | " (Utilities|String|ToString(Float) _w)) true true Color)
  (return))

(fn UpdateTestSphereRotation
  (params (GyroSensor :type GyroSensorEnum%20Enum :default "NewEnumerator0") (QuatRotator :type Quat%20Structure) (SmoothDeltaTime :type Float%20%28single-precision%29) (SmoothInterpSpeed :type Float%20%28single-precision%29))
  (if (Utilities|Enum|Equal(Enum) GyroSensor (Variables|Default|GetCurrentSensor))
    (Transformation|SetActorRotation (Variables|Default|GetTestSphere) (Math|Interpolation|RInterpTo (Transformation|GetActorRotation (Variables|Default|GetTestSphere)) (Class|KismetMathLibrary|QuatRotator QuatRotator) SmoothDeltaTime SmoothInterpSpeed))
    (return)))