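; UDP server actor that receives gyroscope sensor data over the network and passes it to a SensorController.
; It listens on port 8855 from BeginPlay to EndPlay, prints each packet and parses it as JSON.
; For "gyroData" messages, it maps the sensor name to an enum by string comparison and forwards the quaternion.
; Unmatched names fall back to the first enum entry, which is logged as not found.
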(event Custom|UDPReceivedEvent
  (params (Bytes :type Array%20of%20Bytes))
  (bind _returnvalue (Class|CUBlueprintLibrary|ToString(Bytes) Bytes))
  (Development|PrintString _returnvalue true true "(R=0.000000,G=0.660000,B=1.000000,A=1.000000)" 0.1)
  (bind _returnvalue_2 (Class|SIOJsonValue|AsObject (Class|SIOJsonValue|ValuefromJsonString _returnvalue)))
  (if (Utilities|Enum|Equal(Enum) (Class|SIOJsonObject|GetStringField _returnvalue_2 "type") "gyroData")
    (bind _gyrosensorenum (CallFunction|GetGyroSensorEnumfromString (Class|SIOJsonObject|GetStringField _returnvalue_2 "sensorName")))
    (if (Utilities|Enum|Equal(Enum) _gyrosensorenum "NewEnumerator0")
      (Development|PrintString (Utilities|String|Append "Sensor " (Class|SIOJsonObject|GetStringField _returnvalue_2 "sensorName") " not found"))
      (else
        (Default|GyroDataReceive (Variables|Default|GetSensorController) _gyrosensorenum (Utilities|Struct|MakeQuat (Class|SIOJLibrary|ToFloat(JsonValue) (Class|SIOJsonObject|GetField _returnvalue_2 "qX")) (Class|SIOJLibrary|ToFloat(JsonValue) (Class|SIOJsonObject|GetField _returnvalue_2 "qY")) (Class|SIOJLibrary|ToFloat(JsonValue) (Class|SIOJsonObject|GetField _returnvalue_2 "qZ")) (Class|SIOJLibrary|ToFloat(JsonValue) (Class|SIOJsonObject|GetField _returnvalue_2 "qW"))))))))

(event EventBeginPlay
  (bind _udp (Variables|Default|GetUDP))
  (Class|UDPComponent|StartReceiveSocketListening _udp 8855)
  (EventDispatchers|BindEventtoOnReceivedBytes _udp (delegate Custom|UDPReceivedEvent)))

(event EventEndPlay
  (params (EndPlayReason :type EEndPlayReason%20Enum :default "Destroyed"))
  (Class|UDPComponent|CloseReceiveSocket (Variables|Default|GetUDP)))

(fn ConstructionScript)

(fn GetGyroSensorEnumfromString
  (params (GyroSensorString :type String))
  (bind _enumvalue (|ForEachGyroSensorEnum)
    (:LoopBody
      (if (Utilities|Enum|Equal(Enum) (Utilities|String|EnumtoString _enumvalue) GyroSensorString)
        (return _enumvalue)))
    (:then
      (return "NewEnumerator0"))))