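; Sensor controller that turns gyro quaternion readings into bone rotations on a T-pose character for motion capture.
; During calibration it sums a fixed number of samples per sensor, then averages them component-wise into an offset.
; Otherwise it multiplies each inverted reading by that offset and remaps, flips and scales axes using per-sensor bone settings.
; The result goes to the Mixamo mocap Anim Blueprint with smoothing parameters.
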(event Custom|BoneRotation
  (params (GyroSensor :type GyroSensorEnum%20Enum :default "NewEnumerator0") (Quat :type Quat%20Structure))
  ;[0.05517 0.1 1] BoneRotation
  (bind (_gyrosensor _quat) (CallFunction|GetCalibrationRotateOffset GyroSensor Quat))
  (bind (_sensor _quaternion) (CallFunction|SetAxisSettings _gyrosensor _quat))
  (CallFunction|UpdateBoneRotationAnimClass _sensor _quaternion (Variables|Default|GetSmoothDeltaTime) (Variables|Default|GetSmoothInterpSpeed)))

(event Custom|GyroDataReceive
  (params (GyroSensor :type GyroSensorEnum%20Enum :default "NewEnumerator0") (GyroQuaternion :type Quat%20Structure))
  ;[1 0 0.5519] Gyro Data Receive
  (if (Variables|Default|GetisCalibration)
    (Calibration|AddGyroCalibration GyroSensor GyroQuaternion)
    (Development|PrintString "Calibration Process")
    (else
      (CallFunction|BoneRotation GyroSensor GyroQuaternion))))

(fn ConstructionScript)

(fn GetGyroSensorCalibrationStruct
  (params (GyroSensor :type GyroSensorEnum%20Enum :default "NewEnumerator0"))
  (bind _gyrosensorcalibrationstruct (Utilities|Struct|MakeGyroSensorCalibrationStruct 0 "(X=0.000000,Y=0.000000,Z=0.000000,W=1.000000)" false))
  (bind _gyrosensorcalibrationmapstruct (Variables|Default|GetGyroSensorCalibrationMapStruct))
  (bind (_value _returnvalue) (Utilities|Map|Find _gyrosensorcalibrationmapstruct GyroSensor))
  (if _returnvalue
    (return GyroSensor _value)
    (else
      (Utilities|Map|Add _gyrosensorcalibrationmapstruct GyroSensor _gyrosensorcalibrationstruct)
      (return GyroSensor _gyrosensorcalibrationstruct))))

(fn GetSensorBoneEnumfromString
  (params (GyroSensorString :type String))
  (bind _enumvalue (|ForEachGyroSensorEnum)
    (:LoopBody
      (if (Utilities|Enum|Equal(Enum) (Utilities|String|EnumtoString _enumvalue) GyroSensorString)
        (return _enumvalue)))
    (:then
      (return "NewEnumerator0"))))

(fn SetGyroSensorCalibrationStruct
  (params (GyroSensor :type GyroSensorEnum%20Enum :default "NewEnumerator0") (GyroSensorCalibrationStruct :type Gyro%20Sensor%20Calibration%20Struct%20Structure))
  (Utilities|Map|Add (Variables|Default|GetGyroSensorCalibrationMapStruct) GyroSensor GyroSensorCalibrationStruct)
  (return))

(fn AddGyroSensorCalibrationOffset
  (params (GyroSensor :type GyroSensorEnum%20Enum :default "NewEnumerator0") (QuatRotator :type Quat%20Structure))
  (bind (_x _y _z _w) (Utilities|Struct|BreakQuat QuatRotator))
  (bind _gyrosensorcalibrationstruct (Calibration|GetGyroSensorCalibrationStruct GyroSensor))
  (Calibration|SetGyroSensorCalibrationStruct GyroSensor (Utilities|Struct|MakeGyroSensorCalibrationStruct (+ (.GyroSensorCalibrationCount (Utilities|Struct|BreakGyroSensorCalibrationStruct _gyrosensorcalibrationstruct)) 1) (Utilities|Struct|MakeQuat (+ (.X (Utilities|Struct|BreakQuat (.GyroSensorOffsetMap (Utilities|Struct|BreakGyroSensorCalibrationStruct _gyrosensorcalibrationstruct)))) _x) (+ (.Y (Utilities|Struct|BreakQuat (.GyroSensorOffsetMap (Utilities|Struct|BreakGyroSensorCalibrationStruct _gyrosensorcalibrationstruct)))) _y) (+ (.Z (Utilities|Struct|BreakQuat (.GyroSensorOffsetMap (Utilities|Struct|BreakGyroSensorCalibrationStruct _gyrosensorcalibrationstruct)))) _z) (+ (.W (Utilities|Struct|BreakQuat (.GyroSensorOffsetMap (Utilities|Struct|BreakGyroSensorCalibrationStruct _gyrosensorcalibrationstruct)))) _w)) (.GyroSensorCalibrationComplete (Utilities|Struct|BreakGyroSensorCalibrationStruct _gyrosensorcalibrationstruct))))
  (return GyroSensor (Utilities|Struct|MakeGyroSensorCalibrationStruct (+ (.GyroSensorCalibrationCount (Utilities|Struct|BreakGyroSensorCalibrationStruct _gyrosensorcalibrationstruct)) 1) (Utilities|Struct|MakeQuat (+ (.X (Utilities|Struct|BreakQuat (.GyroSensorOffsetMap (Utilities|Struct|BreakGyroSensorCalibrationStruct _gyrosensorcalibrationstruct)))) _x) (+ (.Y (Utilities|Struct|BreakQuat (.GyroSensorOffsetMap (Utilities|Struct|BreakGyroSensorCalibrationStruct _gyrosensorcalibrationstruct)))) _y) (+ (.Z (Utilities|Struct|BreakQuat (.GyroSensorOffsetMap (Utilities|Struct|BreakGyroSensorCalibrationStruct _gyrosensorcalibrationstruct)))) _z) (+ (.W (Utilities|Struct|BreakQuat (.GyroSensorOffsetMap (Utilities|Struct|BreakGyroSensorCalibrationStruct _gyrosensorcalibrationstruct)))) _w)) (.GyroSensorCalibrationComplete (Utilities|Struct|BreakGyroSensorCalibrationStruct _gyrosensorcalibrationstruct)))))

(fn AddGyroCalibration
  (params (GyroSensor :type GyroSensorEnum%20Enum :default "NewEnumerator0") (QuatRotator :type Quat%20Structure))
  (bind _gyrosensorcalibrationstruct (Calibration|GetGyroSensorCalibrationStruct GyroSensor))
  (if (< (.GyroSensorCalibrationCount (Utilities|Struct|BreakGyroSensorCalibrationStruct _gyrosensorcalibrationstruct)) (Variables|Default|GetCalibrationCount))
    (Calibration|AddGyroSensorCalibrationOffset GyroSensor QuatRotator)
    (else
      (Calibration|SetGyroSensorCalibrationCompelte GyroSensor)))
  (Calibration|CheckGyroSensorCalibrationComplete)
  (return))

(fn ResetAllSensorCalibration
  (Utilities|Map|Clear (Variables|Default|GetGyroSensorCalibrationMapStruct))
  (return))

(fn GetSkeletonBoneStructfromSensorBone
  (params (GyroSensor :type GyroSensorEnum%20Enum :default "NewEnumerator0"))
  (bind _sensorskeletonbonemapstruct (Variables|Default|GetSensorSkeletonBoneMapStruct))
  (bind (_value _returnvalue) (Utilities|Map|Find _sensorskeletonbonemapstruct GyroSensor))
  (if _returnvalue
    (return _value)
    (else
      (return (Utilities|Struct|MakeSkeletonBoneStruct "NewEnumerator0" "NewEnumerator0" 1.0 false "NewEnumerator1" 1.0 false "NewEnumerator2" 1.0 false)))))

(fn GetCalibrationRotateOffset
  (params (GyroSensorEnum :type GyroSensorEnum%20Enum :default "NewEnumerator0") (QuatRotator :type Quat%20Structure))
  (bind _gyrosensorcalibrationstruct (Calibration|GetGyroSensorCalibrationStruct GyroSensorEnum))
  (return GyroSensorEnum (Class|KismetMathLibrary|QuatNormalized (* (Class|KismetMathLibrary|QuatInversed QuatRotator) (.GyroSensorOffsetMap (Utilities|Struct|BreakGyroSensorCalibrationStruct _gyrosensorcalibrationstruct))) 0.0001)))

(fn SetAxisSettings
  (params (GyroSensor :type GyroSensorEnum%20Enum :default "NewEnumerator0") (GyroQuaternion :type Quat%20Structure))
  (bind (_x _y _z _w) (Utilities|Struct|BreakQuat GyroQuaternion))
  (bind _skeletonbonestruct (CallFunction|GetSkeletonBoneStructfromSensorBone GyroSensor))
  (switch Utilities|FlowControl|Switch|SwitchonAxisEnum (.axisX (Utilities|Struct|BreakSkeletonBoneStruct _skeletonbonestruct))
    (:NewEnumerator0
      (LocalVariables|SetlocalAxisX _x))
    (:NewEnumerator1
      (LocalVariables|SetlocalAxisX _y))
    (:NewEnumerator2
      (LocalVariables|SetlocalAxisX _z)))
  (switch Utilities|FlowControl|Switch|SwitchonAxisEnum (.axisY (Utilities|Struct|BreakSkeletonBoneStruct _skeletonbonestruct))
    (:NewEnumerator0
      (LocalVariables|SetlocalAxisY _x))
    (:NewEnumerator1
      (LocalVariables|SetlocalAxisY _y))
    (:NewEnumerator2
      (LocalVariables|SetlocalAxisY _z)))
  (switch Utilities|FlowControl|Switch|SwitchonAxisEnum (.axisZ (Utilities|Struct|BreakSkeletonBoneStruct _skeletonbonestruct))
    (:NewEnumerator0
      (LocalVariables|SetlocalAxisZ _x))
    (:NewEnumerator1
      (LocalVariables|SetlocalAxisZ _y))
    (:NewEnumerator2
      (LocalVariables|SetlocalAxisZ _z)))
  (LocalVariables|SetlocalAxisW _w)
  (return GyroSensor (Utilities|Struct|MakeQuat (* (Math|Float|SelectFloat (* (LocalVariables|GetlocalAxisX) -1.0) (LocalVariables|GetlocalAxisX) (.inverseX (Utilities|Struct|BreakSkeletonBoneStruct _skeletonbonestruct))) (.scaleAxisX (Utilities|Struct|BreakSkeletonBoneStruct _skeletonbonestruct))) (* (Math|Float|SelectFloat (* (LocalVariables|GetlocalAxisY) -1.0) (LocalVariables|GetlocalAxisY) (.inverseY (Utilities|Struct|BreakSkeletonBoneStruct _skeletonbonestruct))) (.scaleAxisY (Utilities|Struct|BreakSkeletonBoneStruct _skeletonbonestruct))) (* (Math|Float|SelectFloat (* (LocalVariables|GetlocalAxisZ) -1.0) (LocalVariables|GetlocalAxisZ) (.inverseZ (Utilities|Struct|BreakSkeletonBoneStruct _skeletonbonestruct))) (.scaleAxisZ (Utilities|Struct|BreakSkeletonBoneStruct _skeletonbonestruct))) (LocalVariables|GetlocalAxisW))))

(fn SetGyroSensorCalibrationCompelte
  (params (GyroSensor :type GyroSensorEnum%20Enum :default "NewEnumerator0"))
  (bind (_gyrosensorenum _gyrosensorcalibrationstruct) (Calibration|GetGyroSensorCalibrationStruct GyroSensor))
  (if (.GyroSensorCalibrationComplete (Utilities|Struct|BreakGyroSensorCalibrationStruct _gyrosensorcalibrationstruct))
    (return)
    (else
      (Calibration|SetGyroSensorCalibrationStruct _gyrosensorenum (Utilities|Struct|MakeGyroSensorCalibrationStruct (.GyroSensorCalibrationCount (Utilities|Struct|BreakGyroSensorCalibrationStruct _gyrosensorcalibrationstruct)) (Utilities|Struct|MakeQuat (/ (.X (Utilities|Struct|BreakQuat (.GyroSensorOffsetMap (Utilities|Struct|BreakGyroSensorCalibrationStruct _gyrosensorcalibrationstruct)))) (Math|Conversions|ToFloat(Integer) (Variables|Default|GetCalibrationCount))) (/ (.Y (Utilities|Struct|BreakQuat (.GyroSensorOffsetMap (Utilities|Struct|BreakGyroSensorCalibrationStruct _gyrosensorcalibrationstruct)))) (Math|Conversions|ToFloat(Integer) (Variables|Default|GetCalibrationCount))) (/ (.Z (Utilities|Struct|BreakQuat (.GyroSensorOffsetMap (Utilities|Struct|BreakGyroSensorCalibrationStruct _gyrosensorcalibrationstruct)))) (Math|Conversions|ToFloat(Integer) (Variables|Default|GetCalibrationCount))) (/ (.W (Utilities|Struct|BreakQuat (.GyroSensorOffsetMap (Utilities|Struct|BreakGyroSensorCalibrationStruct _gyrosensorcalibrationstruct)))) (Math|Conversions|ToFloat(Integer) (Variables|Default|GetCalibrationCount)))) true))
      (return))))

(fn CheckGyroSensorCalibrationComplete
  (bind _gyrosensorcalibrationmapstruct (Variables|Default|GetGyroSensorCalibrationMapStruct))
  (bind _keys (Utilities|Map|Keys _gyrosensorcalibrationmapstruct))
  (for _array_element _keys
    (if (not (.GyroSensorCalibrationComplete (Utilities|Struct|BreakGyroSensorCalibrationStruct (.Value (Utilities|Map|Find _gyrosensorcalibrationmapstruct _array_element)))))
      (bind _output_get (LocalVariables|SetlocalCalibrationIsComplete false))
      (Variables|Default|SetisCalibration (not _output_get))
      (return _output_get)))
  (bind _output_get_2 (Variables|Default|SetisCalibration (not (LocalVariables|GetlocalCalibrationIsComplete))))
  (return _output_get_2))

(fn QuatPrintString
  (params (Quat :type Quat%20Structure) (Color :type Linear%20Color%20Structure))
  (bind (_x _y _z _w) (Utilities|Struct|BreakQuat Quat))
  (Development|PrintString (Utilities|String|Append (Utilities|String|ToString(Float) _x) " | " (Utilities|String|ToString(Float) _y) " | " (Utilities|String|ToString(Float) _z) " | " (Utilities|String|ToString(Float) _w)) true true Color)
  (return))

(fn UpdateBoneRotationAnimClass
  (params (GyroSensor :type GyroSensorEnum%20Enum :default "NewEnumerator0") (QuatRotator :type Quat%20Structure) (SmoothDeltaTime :type Float%20%28single-precision%29) (SmoothInterpSpeed :type Float%20%28single-precision%29))
  (bind _skeletonbonestruct (CallFunction|GetSkeletonBoneStructfromSensorBone GyroSensor))
  (bind _asmixamo_mocap_anim_bp (Utilities|Casting|CastToMixamo_Mocap_Anim_BP (Components|SkeletalMesh|GetAnimInstance (Variables|/Script/Engine.Character|GetMesh (Variables|Default|GetTPoseCharacter)))))
  (Default|RotateDataReceive _asmixamo_mocap_anim_bp (.SkeletonBoneEnum (Utilities|Struct|BreakSkeletonBoneStruct _skeletonbonestruct)) (.BoneInitRotate (Utilities|Struct|BreakSkeletonBoneStruct _skeletonbonestruct)) QuatRotator SmoothDeltaTime SmoothInterpSpeed)
  (return))