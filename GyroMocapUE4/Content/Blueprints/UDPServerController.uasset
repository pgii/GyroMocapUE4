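; UDP server Blueprint that receives gyroscope sensor rotations over the network and passes them to the SensorController.
; It listens on a fixed port from BeginPlay until EndPlay, printing each received packet and parsing it as JSON.
; For gyroData messages, it maps the sensor name to a bone enum, builds a quaternion from the string fields and forwards both.
; Unrecognized sensor names print a not-found message instead.
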(event Custom|UDPReceivedEvent
  (params (Bytes :type Array%20of%20Bytes))
  (bind _returnvalue (Class|CUBlueprintLibrary|ToString(Bytes) Bytes))
  (Development|PrintString _returnvalue)
  (bind _returnvalue_2 (Class|SIOJsonValue|AsObject (Class|SIOJsonValue|ValuefromJsonString _returnvalue)))
  (if (Utilities|Enum|Equal(Enum) (Class|SIOJsonObject|GetStringField _returnvalue_2 "type") "gyroData")
    (bind _gyrosensor (Default|GetSensorBoneEnumfromString (Variables|Default|GetSensorController) (Class|SIOJsonObject|GetStringField _returnvalue_2 "sensorName")))
    (if (Utilities|Enum|Equal(Enum) _gyrosensor "NewEnumerator0")
      (Development|PrintString (Utilities|String|Append "Sensor " (Class|SIOJsonObject|GetStringField _returnvalue_2 "sensorName") " not found"))
      (else
        (Default|GyroDataReceive (Variables|Default|GetSensorController) _gyrosensor (Utilities|Struct|MakeQuat (Math|Conversions|ToFloat(Integer) (Class|SIOJsonObject|GetStringField _returnvalue_2 "qX")) (Math|Conversions|ToFloat(Integer) (Class|SIOJsonObject|GetStringField _returnvalue_2 "qY")) (Math|Conversions|ToFloat(Integer) (Class|SIOJsonObject|GetStringField _returnvalue_2 "qZ")) (Math|Conversions|ToFloat(Integer) (Class|SIOJsonObject|GetStringField _returnvalue_2 "qW"))))))))

(event EventBeginPlay
  (bind _udp (Variables|Default|GetUDP))
  (Class|UDPComponent|StartReceiveSocketListening _udp 7755)
  (EventDispatchers|BindEventtoOnReceivedBytes _udp (delegate Custom|UDPReceivedEvent)))

(event EventEndPlay
  (params (EndPlayReason :type EEndPlayReason%20Enum :default "Destroyed"))
  (Class|UDPComponent|CloseReceiveSocket (Variables|Default|GetUDP)))

(fn ConstructionScript)